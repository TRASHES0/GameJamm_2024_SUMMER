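; BP_AI_3 is an enemy that detects the player through pawn sensing and sets the hasSeenPlayer blackboard flag for its AI.
; Touching the player with Hit_Scan calls the player's Hit, plays hurt sounds and destroys the enemy.
; Bubble projectiles hitting the capsule reduce HP, shift a ChangeColor material parameter by lost health, and at zero HP destroy it with death sounds.
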(event `self.PawnSensing.OnSeePawn`
  (params (Pawn :type "Pawn Object Reference"))
  (cast `/Game/Blueprints/Character/BP_MainChar` Pawn)
  (`BlackboardComponent.SetValueAsBool` (`AIBlueprintHelperLibrary.GetBlackboard` (`AIBlueprintHelperLibrary.GetAIController` self)) "hasSeenPlayer" true))

(event `self.Hit_Scan.OnComponentBeginOverlap`
  (params (OverlappedComponent :type "PrimitiveComponent Object Reference") (OtherActor :type "Actor Object Reference") (OtherComp :type "PrimitiveComponent Object Reference") (OtherBodyIndex :type Integer) (bFromSweep :type Boolean) (SweepResult :type "HitResult Structure (by ref)"))
  (bind _asbp_main_char (cast `/Game/Blueprints/Character/BP_MainChar` OtherActor))
  (`/Game/Blueprints/Character/BP_MainChar.Hit` _asbp_main_char)
  (`|ExecutionSequence`
    (:`then_0`
      (`GameplayStatics.PlaySound2D` (`|GetArrayItem` (`self.BadSoundArr`) (`KismetMathLibrary.RandomInteger` 3)) 1.0 1.0 0.0 null null)
      (`self.K2_DestroyActor`))
    (:`then_1`
      (`GameplayStatics.PlaySound2D` "/Game/Sound/DamagedSound.DamagedSound" 1.0 1.0 0.0 null null))))

(event `self.CapsuleComponent.OnComponentBeginOverlap`
  (params (OverlappedComponent :type "PrimitiveComponent Object Reference") (OtherActor :type "Actor Object Reference") (OtherComp :type "PrimitiveComponent Object Reference") (OtherBodyIndex :type Integer) (bFromSweep :type Boolean) (SweepResult :type "HitResult Structure (by ref)"))
  (bind _asbp_bubble_1 (cast `/Game/Material/BP_Bubble_1` OtherActor))
  (set `self.HP` (- (`self.HP`) (`/Game/Material/BP_Bubble_1.Damage` _asbp_bubble_1)))
  (`self.K2_DestroyActor` _asbp_bubble_1)
  (`self.ChangeColor`)
  (`self.CheckDeath`))

(fn `ChangeColor`
  (`MeshComponent.SetScalarParameterValueOnMaterials` (`self.Mesh`) "ChangeColor" (- 1.0 (/ (`self.HP`) 100.0))))

(fn `CheckDeath`
  (if (<= (`self.HP`) 0.0)
    (`|ExecutionSequence`
      (:`then_0`
        (`GameplayStatics.PlaySound2D` (`|GetArrayItem` (`self.GoodSoundArr`) (`KismetMathLibrary.RandomInteger` 3)) 1.0 1.0 0.0 null null)
        (`self.K2_DestroyActor`))
      (:`then_1`
        (`GameplayStatics.PlaySound2D` "/Game/Sound/EnemyDieSound.EnemyDieSound" 1.0 1.0 0.0 null null)))))

(fn `UserConstructionScript`)
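; BP_PatrolRoute is a spline-based patrol route actor in the boss AI folder.
; IncrementPatrolRoute steps an index along the spline points, flipping direction at the last point and at the first for a back-and-forth path.
; GetSplinePointsWorldLocation returns the current point's location, sampled in Local coordinate space despite its name.
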(event `IncrementPatrolRoute`
  (bind _output_get (set `self.Index` (+ (`self.Index`) (`self.Drection`))))
  (if (== _output_get (- (`SplineComponent.GetNumberOfSplinePoints` (`self.PatrolRoute`)) 1))
    (set `self.Drection` -1)
    (elif (== (`self.Index`) 0)
      (set `self.Drection` 1))))

(fn `GetSplinePointsWorldLocation`
  (returns (NextLocation :type "Vector Structure"))
  (return (`SplineComponent.GetLocationAtSplinePoint` (`self.PatrolRoute`) (`self.Index`) "Local")))

(fn `UserConstructionScript`)
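; Boss enemy character that attacks the player and exposes patrol route, range and movement speed functions.
; Attack plays a placeholder Test montage, and its notify fires a debug-drawn forward sphere trace for pawns that calls Hit on BP_MainChar.
; Montage completion or interruption both call OnAttackEnd to signal that the attack is over.
; Helper functions return fixed attack and defense radii and the patrol route, and switch max walk speed between walk and run.
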(event `Attack`
  (bind _returnvalue (`self.K2_GetActorLocation`))
  (bind _notifyname (`|PlayMontage` (`self.Mesh`) "/Game/ControlRig/Characters/Mannequins/Animations/Quinn/Test.Test")
    (:`OnCompleted`
      (`self.OnAttackEnd` :!label _label))
    (:`OnInterrupted`
      (goto _label))
    (:`OnNotifyBegin`
      (switch `name` _notifyname
        (:`Attack`
          (bind (_outhit _returnvalue_2) (`KismetSystemLibrary.SphereTraceSingleForObjects` :`Start` _returnvalue :`End` (+ _returnvalue (* (`self.GetActorForwardVector`) 220.0)) :`Radius` 100.0 :`ObjectTypes` (`|MakeArray` "ObjectTypeQuery3" :!type "EObjectTypeQuery Enum") :`DrawDebugType` "ForDuration" :`DrawTime` 10.0))
          (if _returnvalue_2
            (bind _asbp_main_char (cast `/Game/Blueprints/Character/BP_MainChar` (`.HitActor` (`GameplayStatics.BreakHitResult` _outhit))))
            (`/Game/Blueprints/Character/BP_MainChar.Hit` _asbp_main_char)))))))

(fn `GetIdelRange`
  (returns (AttackRadius :type "Float (double-precision)") (DefenseRadius :type "Float (double-precision)"))
  (return 150.0 600.0))

(fn `GetPatrolRoute`
  (returns (NewParam :type "/Game/AI/AI_Boss/BP_PatrolRoute Object Reference"))
  (return (`self.PatrolRoute`)))

(fn `SetMovementSpeed`
  (params (Movement :type "/Game/AI/AI_Boss/BTT/E_MoveSpeed Enum" :default "NewEnumerator0"))
  (returns (Speed :type "Float (double-precision)"))
  (set `CharacterMovementComponent.MaxWalkSpeed` (select `/Game/AI/AI_Boss/BTT/E_MoveSpeed` Movement :`NewEnumerator0` 300.0 :`NewEnumerator1` 600.0 :!type "Float (single-precision)") (`self.CharacterMovement`))
  (return 0.0))

(fn `UserConstructionScript`)
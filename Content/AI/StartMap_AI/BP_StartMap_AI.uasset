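; BP_StartMap_AI is a start map AI pawn that endlessly patrols waypoints at a slow walk speed.
; BeginPlay starts PatrolWayPoint, which sets the walk speed and runs AIMoveTo to the current WayPoints entry.
; On success, it pauses briefly and re-calls itself before advancing Index, which wraps after two points.
; Failed moves have no handler, and the overlap event is empty.
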(event `self.ReceiveBeginPlay`
  (`self.PatrolWayPoint`))

(event `PatrolWayPoint`
  ;[1 1 1] patrol
  (set `CharacterMovementComponent.MaxWalkSpeed` 150.0 (`self.CharacterMovement`))
  (`|AIMoveTo` self (`|GetArrayItem` (`self.WayPoints`) (`self.Index`)) null
    (:`OnSuccess`
      (`KismetSystemLibrary.Delay` 1.5)
      (`self.PatrolWayPoint`)
      (`/Engine/EditorBlueprintResources/StandardMacros.IncrementInt` (`self.Index`)
        (:`  `
          (if (== (`self.Index`) 2)
            (set `self.Index` 0)))))))

(fn `UserConstructionScript`)
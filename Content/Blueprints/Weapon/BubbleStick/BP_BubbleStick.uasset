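; Bubble stick weapon that sprays bubbles while fired and damages AI enemies in front of it.
; LaunchWeapon activates the Bubble component on click and deactivates it otherwise.
; After a brief delay, it runs a forward capsule trace from Bubble, with reach growing with elapsed time up to a fixed cap.
; Each BP_AI hit loses HP by Damage, changes color and checks for death.
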(event `self.Launch_Weapon`
  (params (isClicked :type Boolean) (ElapsedTime :type "Float (double-precision)") (TriggeredTime :type "Float (double-precision)"))
  (bind _bubble (`self.Bubble`))
  (bind _bubble_2 (`self.Bubble`))
  (bind _returnvalue (`SceneComponent.GetForwardVector` _bubble_2))
  (bind _returnvalue_2 (`SceneComponent.K2_GetComponentLocation` _bubble_2))
  (bind _returnvalue_3 (+ (* ElapsedTime 50.0) 50.0))
  (if isClicked
    (`ActorComponent.Activate` _bubble false)
    (`KismetSystemLibrary.Delay` 0.1)
    (if (<= _returnvalue_3 150.0)
      (bind _outhits (`KismetSystemLibrary.CapsuleTraceMulti` :`Start` _returnvalue_2 :`End` (+ _returnvalue_2 (* _returnvalue _returnvalue_3)) :`Radius` 50.0 :`HalfHeight` 10.0 :`TraceChannel` "TraceTypeQuery1" :`DrawTime` 1.0))
      (for _array_element _outhits
        (bind _asbp_ai (cast `/Game/AI/Enemy_AI/BP_AI` (`.HitActor` (`GameplayStatics.BreakHitResult` _array_element))))
        (set `/Game/AI/Enemy_AI/BP_AI.HP` (- (`/Game/AI/Enemy_AI/BP_AI.HP` _asbp_ai) (`self.Damage`)) _asbp_ai)
        (`/Game/AI/Enemy_AI/BP_AI.ChangeColor` _asbp_ai)
        (`/Game/AI/Enemy_AI/BP_AI.CheckDeath` _asbp_ai))
      (else
        (bind _outhits_2 (`KismetSystemLibrary.CapsuleTraceMulti` :`Start` _returnvalue_2 :`End` (+ _returnvalue_2 (* _returnvalue 150.0)) :`Radius` 50.0 :`HalfHeight` 10.0 :`TraceChannel` "TraceTypeQuery1" :`DrawTime` 1.0))
        (for _array_element_2 _outhits_2
          (bind _asbp_ai_2 (cast `/Game/AI/Enemy_AI/BP_AI` (`.HitActor` (`GameplayStatics.BreakHitResult` _array_element_2))))
          (set `/Game/AI/Enemy_AI/BP_AI.HP` (- (`/Game/AI/Enemy_AI/BP_AI.HP` _asbp_ai_2) (`self.Damage`)) _asbp_ai_2)
          (`/Game/AI/Enemy_AI/BP_AI.ChangeColor` _asbp_ai_2)
          (`/Game/AI/Enemy_AI/BP_AI.CheckDeath` _asbp_ai_2))))
    (else
      (`ActorComponent.Deactivate` _bubble))))

(fn `UserConstructionScript`
  (`parent.UserConstructionScript`))
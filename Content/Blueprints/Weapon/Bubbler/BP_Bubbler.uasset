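; Bubbler weapon Blueprint that fires a chargeable bubble projectile.
; LaunchWeapon acts only when IsClicked is false, spawning a BP_Bubble_1 at the static mesh's FireSocket.
; ElapsedTime drives both the bubble's scale and its multiplier on the weapon's Damage, so a larger value gives a bigger, stronger shot.
; The bubble's projectile movement velocity is set along the socket's forward vector at a fixed speed.
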(event `self.Launch_Weapon`
  (params (isClicked :type Boolean) (ElapsedTime :type "Float (double-precision)") (TriggeredTime :type "Float (double-precision)"))
  (bind (_returnvalue_location _returnvalue_rotation) (`KismetMathLibrary.BreakTransform` (`SceneComponent.GetSocketTransform` (`self.StaticMesh`) "FireSocket" "RTS_World")))
  (if (not isClicked)
    (bind _returnvalue (`|SpawnActorFromClass` "/Game/Material/BP_Bubble_1.BP_Bubble_1_C" (`KismetMathLibrary.MakeTransform` _returnvalue_location _returnvalue_rotation (* (`KismetMathLibrary.Vector_One`) (+ ElapsedTime 0.5))) "Undefined" "MultiplyWithRoot" null null))
    (set `/Game/Material/BP_Bubble_1.Damage` (* (+ ElapsedTime 1.0) (`self.Damage`)) _returnvalue)
    (set `MovementComponent.Velocity` (* (`KismetMathLibrary.GetForwardVector` _returnvalue_rotation) 2000.0) (`/Game/Material/BP_Bubble_1.ProjectileMovement` _returnvalue))))

(fn `UserConstructionScript`
  (`parent.UserConstructionScript`))
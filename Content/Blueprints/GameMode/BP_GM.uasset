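; BP_GM is a game mode Blueprint that drives level transitions for the game.
; SpawnBoss increments a Point counter and, when it reaches fifteen, opens the Boss_Level after a short delay rather than spawning an actor.
; End and ReStart are events that open EndRoom and Main_Level after brief delays.
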(event `SpawnBoss`
  (set `self.Point` (+ (`self.Point`) 1))
  (if (== (`self.Point`) 15)
    (`KismetSystemLibrary.Delay` 1.0)
    (`GameplayStatics.OpenLevel` "Boss_Level")))

(event `End`
  (`KismetSystemLibrary.Delay` 1.0)
  (`GameplayStatics.OpenLevel` "EndRoom"))

(event `ReStart`
  (`KismetSystemLibrary.Delay` 0.3)
  (`GameplayStatics.OpenLevel` "Main_Level"))

(fn `UserConstructionScript`)